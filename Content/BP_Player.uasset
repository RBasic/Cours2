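; BP_Player is a player blueprint with tap-to-jump, Flappy Bird-style movement on a physics-driven cube.
; BeginPlay registers the Enhanced Input mapping context.
; Each jump press enables physics, zeroes velocity, applies a fixed upward velocity-change impulse for consistent hops, and sets StartGame.
; Tick maps the cube's clamped vertical velocity to pitch, tilting it as it rises and falls, with roll and yaw zeroed.
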(event Input|EnhancedActionEvents|EnhancedInputActionIA_Jump
  (params (ActionValue :type Boolean) (ElapsedSeconds :type Float%20%28double-precision%29) (TriggeredSeconds :type Float%20%28double-precision%29) (InputAction :type Input%20Action%20Object%20Reference :default "/Game/Inputs/Actions/IA_Jump.IA_Jump"))
  (bind _cube (Variables|Default|GetCube))
  (:Started
    (Physics|SetSimulatePhysics (Variables|Default|GetCube) true)
    (Physics|SetPhysicsLinearVelocity _cube "0, 0, 0" false "None")
    (Physics|AddImpulse _cube "0.000000,0.000000,1000.000000" "None" true)
    (Variables|Default|SetbStartGame true)))

(event EventTick
  (params (DeltaSeconds :type Float%20%28single-precision%29))
  (bind _cube (Variables|Default|GetCube))
  (Transformation|SetWorldRotation _cube (Math|Rotator|MakeRotator 0.0 (Math|Float|MapRangeClamped (.z (Transformation|GetComponentVelocity _cube)) -9e+02 9e+02 -45.0 45.0) 0.0) false false))

(event EventBeginPlay
  (bind _asplayer_controller (Utilities|Casting|CastToPlayerController (Pawn|GetController)))
  (Input|AddMappingContext (PlayerController|LocalPlayerSubsystems|GetEnhancedInputLocalPlayerSubsystem _asplayer_controller) "/Game/Inputs/IMC_Player.IMC_Player" 0 "(bIgnoreAllPressedKeysUntilRelease=True,bForceImmediately=False,bNotifyUserSettings=False)"))

(fn ConstructionScript)